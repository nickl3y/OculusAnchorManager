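; VR player character that calibrates its position and yaw against two saved Oculus spatial anchors, putting anchor1 at the world origin.
; The local client spawns a calibration manager after a delay, loads anchors, and calibrates on success or left menu input.
; The corrected transform replicates through a server-to-multicast refresh.
; It also yaws from right cursor input, shows camera-facing transform debug text, and destroys itself when unpossessed.
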(event `self.ReceiveBeginPlay`
  (`|ExecutionSequence`
    (:`then_0`
      (`HeadMountedDisplayFunctionLibrary.SetTrackingOrigin` "Floor")
      (bind _asplayer_controller (cast `PlayerController` (`self.GetController`)))
      (`EnhancedInputSubsystemInterface.AddMappingContext` (pcsubsystem `EnhancedInputLocalPlayerSubsystem` _asplayer_controller) "/Game/SampleGame/Demo/Input/IMC_Menu.IMC_Menu" 0 (struct)))
    (:`then_1`
      (`KismetSystemLibrary.Delay` 2.0)
      (if (`self.IsLocallyControlled`)
        (bind _returnvalue (`|SpawnActorFromClass` "/Game/SampleGame/Demo/OculusCalibrationManager_Demo.OculusCalibrationManager_Demo_C" (`KismetMathLibrary.MakeTransform` (0.0 0.0 0.0)) "Undefined" "MultiplyWithRoot" null "/Game/SampleGame/Demo/BP_Anchor_Visual.BP_Anchor_Visual_C" null))
        (bind _output_get (set `self.CallibrationManager` _returnvalue))
        (add `/Game/CalibrationNodes/OculusCalibrationManager.AnchorsLoaded` (`self.CallibrationManager`) (delegate `AnchorsLoaded_Event`))
        (`/Game/CalibrationNodes/OculusCalibrationManager.LoadAnchors` _output_get)))))

(event `AnchorsLoaded_Event`
  (params (Successful :type Boolean))
  (if Successful
    (remove `/Game/CalibrationNodes/OculusCalibrationManager.AnchorsLoaded` (`self.CallibrationManager`) (delegate `AnchorsLoaded_Event`))
    (`self.CalibrateVRCharacter`)))

(event `Multicast_RefreshPosition`
  (params (NewTransform :type "Transform Structure (by ref)"))
  (`self.SetActorRotationVR` (.rotation NewTransform))
  (`self.K2_SetActorLocation` (.location NewTransform)))

(event `Client_RefreshCharacterPosition`
  (bind _returnvalue (`KismetMathLibrary.MakeTransform` (`self.K2_GetActorLocation`) (`self.GetVRRotation`)))
  (`/Engine/EditorBlueprintResources/ActorMacros.Switch Has Authority`
    (:`Authority`
      (`self.Multicast_RefreshPosition` _returnvalue))
    (:`Remote`
      (`self.Server_RefreshPosition` _returnvalue))))

(event `Server_RefreshPosition`
  (params (NewTransform :type "Transform Structure (by ref)"))
  (`self.Multicast_RefreshPosition` NewTransform))

(event `EnhancedInput|/Game/SampleGame/Demo/Input/Actions/IA_Menu_Interact_Right`
  (params (ActionValue :type Boolean) (ElapsedSeconds :type "Float (double-precision)") (TriggeredSeconds :type "Float (double-precision)") (InputAction :type "InputAction Object Reference" :default "/Game/SampleGame/Demo/Input/Actions/IA_Menu_Interact_Right.IA_Menu_Interact_Right")))

(event `EnhancedInput|/Game/SampleGame/Demo/Input/Actions/IA_Menu_Interact_Left`
  (params (ActionValue :type Boolean) (ElapsedSeconds :type "Float (double-precision)") (TriggeredSeconds :type "Float (double-precision)") (InputAction :type "InputAction Object Reference" :default "/Game/SampleGame/Demo/Input/Actions/IA_Menu_Interact_Left.IA_Menu_Interact_Left"))
  (:`Started`
    (if ActionValue
      (`self.CalibrateVRCharacter`))))

(event `self.ReceiveUnpossessed`
  (params (OldController :type "Controller Object Reference"))
  (`parent.ReceiveUnpossessed` OldController)
  (`self.K2_DestroyActor`))

(event `self.ReceiveTick`
  (params (DeltaSeconds :type "Float (single-precision)"))
  (`parent.ReceiveTick` DeltaSeconds)
  (`SceneComponent.K2_SetWorldRotation` (`self.TextRender`) (`KismetMathLibrary.FindLookAtRotation` (`SceneComponent.K2_GetComponentLocation` (`self.TextRender`)) (`PlayerCameraManager.GetCameraLocation` (`GameplayStatics.GetPlayerCameraManager` 0))) false false)
  (`TextRenderComponent.K2_SetText` (`self.TextRender`) (`|FormatText` " location={location} \nrotation={rotation} \nVRLoc={VRL} \nVRRot={VRR}" (`KismetStringLibrary.Conv_VectorToString` (`self.K2_GetActorLocation`)) (`KismetStringLibrary.Conv_RotatorToString` (`self.K2_GetActorRotation`)) (`KismetStringLibrary.Conv_VectorToString` (`self.GetVRLocation`)) (`KismetStringLibrary.Conv_RotatorToString` (`self.GetVRRotation`)))))

(event `EnhancedInput|/Game/SampleGame/Demo/Input/Actions/IA_Menu_Cursor_Right`
  (params (ActionValue :type "Vector2D Structure") (ElapsedSeconds :type "Float (double-precision)") (TriggeredSeconds :type "Float (double-precision)") (InputAction :type "InputAction Object Reference" :default "/Game/SampleGame/Demo/Input/Actions/IA_Menu_Cursor_Right.IA_Menu_Cursor_Right"))
  (:`Triggered`
    (`self.SetActorRotationVR` (`KismetMathLibrary.MakeRotator` 0.0 0.0 (+ (.yaw (`self.K2_GetActorRotation`)) (`KismetMathLibrary.BreakVector2D` ActionValue))) true false false)))

(fn `CalibrateVRCharacter`
  (locals (anchor1_transform :type "Transform Structure") (anchor2_transform :type "Transform Structure") (anchors_target_rotation :type "Rotator Structure" :default (struct)))
  (bind (_returnvalue_roll _returnvalue_pitch _returnvalue_yaw) (`KismetMathLibrary.BreakRotator` (`self.GetVRRotation`)))
  (bind _anchor1_transform_location (`KismetMathLibrary.BreakTransform` (`local.anchor1_transform`)))
  (bind (_anchors_target_rotation_roll _anchors_target_rotation_pitch _anchors_target_rotation_yaw) (`KismetMathLibrary.BreakRotator` (`local.anchors_target_rotation`)))
  (bind _actor (`/Game/CalibrationNodes/OculusCalibrationManager.GetAnchorByName` (`self.CallibrationManager`) "anchor1"))
  (set `local.anchor1_transform` (`self.GetTransform` _actor))
  (bind _actor_2 (`/Game/CalibrationNodes/OculusCalibrationManager.GetAnchorByName` (`self.CallibrationManager`) "anchor2"))
  (set `local.anchor2_transform` (`self.GetTransform` _actor_2))
  (set `local.anchors_target_rotation` (`KismetMathLibrary.FindLookAtRotation` (.location (`local.anchor1_transform`)) (.location (`local.anchor2_transform`))))
  (`self.SetActorRotationVR` (`KismetMathLibrary.MakeRotator` 0.0 0.0 (- _returnvalue_yaw _anchors_target_rotation_yaw)))
  (`self.K2_SetActorLocation` (* (- (`self.K2_GetActorLocation`) _anchor1_transform_location) (1.0 1.0 0.0)) false true)
  (`self.Client_RefreshCharacterPosition`)
  (return))

(fn `GetCharacterRotatedPosition`
  (params (OriginalLocation :type "Vector Structure") (DeltaRotation :type "Rotator Structure") (PivotPoint :type "Vector Structure"))
  (returns (OutNewPosition :type "Vector Structure") (OutRotation :type "Rotator Structure"))
  (locals (RotationToUse :type "Rotator Structure") (NewLocationOffset :type "Vector Structure") (NewRotation :type "Rotator Structure"))
  (bind (_newlocation _newrotation) (`VRExpansionFunctionLibrary.RotateAroundPivot` DeltaRotation OriginalLocation (`self.K2_GetActorRotation`) (`KismetMathLibrary.InverseTransformLocation` (`self.GetTransform`) PivotPoint)))
  (return _newlocation _newrotation))

(fn `UserConstructionScript`)