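; Player state for the Shared Spaces spatial anchor sample that relays colocation actions between clients and the server.
; After a replication delay, the local player sends its Oculus net ID to the server, which multicasts so each client's pawn re-shares its anchors.
; Server-to-multicast RPC pairs also distribute anchor UUIDs for loading and teleport pawns to align with an anchor.
; Further server RPCs spawn and explode cubes.
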(event `self.ReceiveBeginPlay`
  ;[1 1 1] Wait for replication to get local player state
  (`KismetSystemLibrary.Delay` 2.0)
  (if (== (`Controller.PlayerState` (`GameplayStatics.GetPlayerController` 0)) self)
    ;[1 1 1] Update the oculus net ID on the server
    (bind _returnvalue (`SharedAnchorsSampleBPLibrary.GetLocalPlayerOculusNetID`))
    (bind _output_get (set `self.OculusNetID` _returnvalue))
    (`self.Server_SetOculusNetID` _output_get)))

(event `Server_SetOculusNetID`
  (params (NetID :type String))
  (set `self.OculusNetID` NetID)
  (`self.NetMutlicast_NewPlayerJoined`))

(event `NetMutlicast_NewPlayerJoined`
  (bind _asbp_vrpawn (cast `/Game/SpatialAnchorsSample/Blueprints/BP_VRPawn` (`GameplayStatics.GetPlayerPawn` 0)))
  (bind _spatialanchormanager_ac (`/Game/SpatialAnchorsSample/Blueprints/BP_VRPawn.SpatialAnchorManager_AC` _asbp_vrpawn))
  (`/Game/SpatialAnchorsSample/Blueprints/Components/BP_SpatialAnchorManagerComponent.ShareSpecifiedAnchors` _spatialanchormanager_ac (`/Game/SpatialAnchorsSample/Blueprints/Components/BP_SpatialAnchorManagerComponent.SharedAnchors` _spatialanchormanager_ac)))

(event `Server_ShareIDs`
  (params (UUIDs :type "Array of OculusXRUUID Structure"))
  (`self.NetMutlicast_ShareAnchors` UUIDs))

(event `NetMutlicast_ShareAnchors`
  (params (UUIDs :type "Array of OculusXRUUID Structure"))
  (bind _returnvalue (`GameplayStatics.GetPlayerPawn` 0))
  (bind _returnvalue_2 (`self.GetComponentByClass` _returnvalue "/Game/SpatialAnchorsSample/Blueprints/Components/BP_SpatialAnchorManagerComponent.BP_SpatialAnchorManagerComponent_C"))
  (`/Engine/EditorBlueprintResources/StandardMacros.IsValid` _returnvalue
    (:`Is Valid`
      (`/Engine/EditorBlueprintResources/StandardMacros.IsValid` _returnvalue_2
        (:`Is Valid`
          (`/Game/SpatialAnchorsSample/Blueprints/Components/BP_SpatialAnchorManagerComponent.GetAllSharedAnchors` _returnvalue_2 UUIDs))))))

(event `Server_OrientToAnchor`
  (params (Position :type "Vector Structure") (Rotation :type "Rotator Structure"))
  (bind _pawnprivate (`self.PawnPrivate`))
  (`self.K2_SetActorLocation` _pawnprivate Position false true)
  (`self.K2_SetActorRotation` _pawnprivate Rotation true)
  (`self.NetMulticast_SetPosition` Position Rotation))

(event `NetMulticast_SetPosition`
  (params (Position :type "Vector Structure") (Rotation :type "Rotator Structure"))
  (bind _pawnprivate (`self.PawnPrivate`))
  (`self.K2_SetActorLocation` _pawnprivate Position false true)
  (`self.K2_SetActorRotation` _pawnprivate Rotation true))

(event `Server_SpawnCube`
  (params (Position :type "Vector Structure"))
  (`|SpawnActorFromClass` "/Game/SpatialAnchorsSample/Blueprints/BP_Cube.BP_Cube_C" (`KismetMathLibrary.MakeTransform` Position (struct) (0.25 0.25 0.25)) "Undefined" "OverrideRootScale" null null))

(event `Server_ThrowCube`
  (params (Cube :type "/Game/SpatialAnchorsSample/Blueprints/BP_Cube Object Reference"))
  (`/Game/SpatialAnchorsSample/Blueprints/BP_Cube.Explode Cube` Cube))

(fn `UserConstructionScript`)