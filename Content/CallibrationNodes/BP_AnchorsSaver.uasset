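; BP_AnchorsSaver manages loading, creating and saving the BP_AnchorsSaveGame object that backs the anchors save slot.
; LoadOrCreateSaveGame returns the cached object if valid, otherwise loads it from the slot or creates a new one when no save exists.
; SaveGame writes the cached object back to the same slot, and does nothing if that object is not valid.
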(fn `LoadOrCreateSaveGame`
  (returns (Output_Get :type "/Game/CallibrationNodes/BP_AnchorsSaveGame Object Reference"))
  (`/Engine/EditorBlueprintResources/StandardMacros.IsValid` (`self.SaveGameObject`)
    (:`Is Valid`
      (return (`self.SaveGameObject`)))
    (:`Is Not Valid`
      (bind _returnvalue (`GameplayStatics.DoesSaveGameExist` (`self.AnchorsSlot`)))
      (if _returnvalue
        (bind _returnvalue_2 (`GameplayStatics.LoadGameFromSlot` (`self.AnchorsSlot`)))
        (bind _asbp_anchors_save_game (cast `/Game/CallibrationNodes/BP_AnchorsSaveGame` _returnvalue_2))
        (bind _output_get (set `self.SaveGameObject` _asbp_anchors_save_game))
        (return _output_get)
        (else
          (bind _returnvalue_3 (`GameplayStatics.CreateSaveGameObject` "/Game/CallibrationNodes/BP_AnchorsSaveGame.BP_AnchorsSaveGame_C"))
          (bind _output_get_2 (set `self.SaveGameObject` _returnvalue_3))
          (return _output_get_2))))))

(fn `SaveGame`
  (bind _savegameobject (`self.SaveGameObject`))
  (`/Engine/EditorBlueprintResources/StandardMacros.IsValid` _savegameobject
    (:`Is Valid`
      (`GameplayStatics.SaveGameToSlot` _savegameobject (`self.AnchorsSlot`)))))