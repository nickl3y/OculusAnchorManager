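; Calibration pawn that drives a selection menu hosted in its Widget component.
; On BeginPlay it caches the WBP_SelectionMenu instance and adds the IMC_Menu Enhanced Input mapping context to its player controller.
; Right cursor input is passed to the menu's UpdateTranslation with Y inverted while triggered, and as zero when ongoing, canceled or completed.
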(event `self.ReceiveBeginPlay`
  (`parent.ReceiveBeginPlay`)
  (`|ExecutionSequence`
    (:`then_0`
      (bind _aswbp_selection_menu (cast `/Game/CallibrationNodes/WBP_SelectionMenu` (`WidgetComponent.GetWidget` (`self.Widget`))))
      (set `self.As WBP Selection Menu` _aswbp_selection_menu))
    (:`then_1`
      (bind _asplayer_controller (cast `PlayerController` (`self.GetController`)))
      (`EnhancedInputSubsystemInterface.AddMappingContext` (pcsubsystem `EnhancedInputLocalPlayerSubsystem` _asplayer_controller) "/Game/VRTemplate/Input/IMC_Menu.IMC_Menu" 0 (struct)))))

(event `EnhancedInput|/Game/VRTemplate/Input/Actions/IA_Menu_Cursor_Right`
  (params (ActionValue :type "Vector2D Structure") (ElapsedSeconds :type "Float (double-precision)") (TriggeredSeconds :type "Float (double-precision)") (InputAction :type "InputAction Object Reference" :default "/Game/VRTemplate/Input/Actions/IA_Menu_Cursor_Right.IA_Menu_Cursor_Right"))
  (:`Triggered`
    (`/Engine/EditorBlueprintResources/StandardMacros.IsValid` (`self.As WBP Selection Menu`)
      (:`Is Valid`
        (`/Game/CallibrationNodes/WBP_SelectionMenu.UpdateTranslation` (`self.As WBP Selection Menu`) (* ActionValue (1.0 -1.0))))))
  (:`Ongoing`
    (`/Engine/EditorBlueprintResources/StandardMacros.IsValid` (`self.As WBP Selection Menu`) :!label _label
      (:`Is Valid`
        (`/Game/CallibrationNodes/WBP_SelectionMenu.UpdateTranslation` (`self.As WBP Selection Menu`) (0.0 0.0)))))
  (:`Canceled`
    (goto _label))
  (:`Completed`
    (goto _label)))

(event `EnhancedInput|/Game/VRTemplate/Input/Actions/IA_Menu_Cursor_Left`
  (params (ActionValue :type "Vector2D Structure") (ElapsedSeconds :type "Float (double-precision)") (TriggeredSeconds :type "Float (double-precision)") (InputAction :type "InputAction Object Reference" :default "/Game/VRTemplate/Input/Actions/IA_Menu_Cursor_Left.IA_Menu_Cursor_Left")))

(fn `UserConstructionScript`)